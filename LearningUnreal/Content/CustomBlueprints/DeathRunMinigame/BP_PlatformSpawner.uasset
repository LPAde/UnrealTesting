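; Platform spawner for the DeathRun minigame that builds a grid of BP_Platform actors and places a BP_Goal after it.
; One tick after BeginPlay, it spawns platforms at a fixed height, stepping along Y and advancing in X every RowAmount platforms.
; Each platform is initialized with a random index into the Materials array.
; The goal spawns at the final column position, one Y offset from the minimum.
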(event EventBeginPlay
  (Utilities|FlowControl|DelayUntilNextTick)
  (for _index (range 1 (Variables|Default|GetSpawnAmount))
    (bind _returnvalue (Game|SpawnActorfromClass "/Game/CustomBlueprints/DeathRunMinigame/BP_Platform.BP_Platform_C" (Math|Transform|MakeTransform (Math|Vector|MakeVector (+ (Variables|Default|GetMinXValue) (* (Variables|Default|GetXOffset) (Variables|Default|GetColumnIndex))) (+ (Variables|Default|GetMinYValue) (* (Variables|Default|GetYOffset) (Variables|Default|GetRowIndex))) (Variables|Default|GetZSpawnValue)) "0, 0, 0" "1.000000,1.000000,1.000000") "AdjustIfPossibleButAlwaysSpawn" "MultiplyWithRoot" 0 0))
    (Default|InitializePlatform _returnvalue (Math|Random|RandomIntegerinRange 0 (- (Utilities|Array|Length (Variables|Default|GetMaterials)) 1)))
    (if (and (== (Math|Integer|%(Integer) _index (Variables|Default|GetRowAmount)) 0) (!= (Variables|Default|GetRowAmount) 0))
      (Math|Integer|IncrementInt (Variables|Default|GetColumnIndex)
        (:%20%20
          (Variables|Default|SetRowIndex 0)))
      (else
        (Math|Integer|IncrementInt (Variables|Default|GetRowIndex)))))
  (Game|SpawnActorfromClass "/Game/CustomBlueprints/DeathRunMinigame/BP_Goal.BP_Goal_C" (Math|Transform|MakeTransform (Math|Vector|MakeVector (+ (Variables|Default|GetMinXValue) (* (Variables|Default|GetXOffset) (Variables|Default|GetColumnIndex))) (+ (Variables|Default|GetMinYValue) (Variables|Default|GetYOffset)) (Variables|Default|GetZSpawnValue)) "0, 0, 0" "1.000000,1.000000,1.000000") "AdjustIfPossibleButAlwaysSpawn" "MultiplyWithRoot" 0 0))

(fn ConstructionScript)