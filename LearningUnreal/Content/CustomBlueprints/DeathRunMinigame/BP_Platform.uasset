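; BP_Platform is a Death Run minigame platform that makes a round trip between a start and a bottom position.
; InitializePlatform applies a material by ID and subscribes the platform to the GameInstance's PlatformManager under that material.
; MovePlatform plays a Timeline that lerps the location, setting its play rate when Speed differs from BaseSpeed.
; A FinishedOnce flag reverses the Timeline after the descent and stops it after the return.
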(event Custom|MovePlatform
  (params (Speed :type Float%20%28double-precision%29))
  (if (== Speed (Variables|Default|GetBaseSpeed))
    (bind _alpha (Timeline|Timeline Play)
      (:Update
        ;[0.15 0.15 0.15 0.5] Moving the platform
        (Transformation|SetWorldLocation (Variables|Default|GetPlatform) (Math|Vector|Lerp(Vector) (Transformation|GetWorldLocation (Variables|Default|GetStartPos)) (Transformation|GetWorldLocation (Variables|Default|GetBottomPos)) _alpha) false false))
      (:Finished
        ;[0.15 0.15 0.15 0.5] Switching between upwards and downwards movement
        (if (Variables|Default|GetFinishedOnce)
          (Variables|Default|SetFinishedOnce false)
          (else
            (Variables|Default|SetFinishedOnce true)
            (Timeline|Timeline ReverseFromEnd)))))
    (else
      (Components|Timeline|SetPlayRate (Variables|Default|GetTimeline) Speed)
      (Timeline|Timeline Play))))

(event Custom|InitializePlatform
  (params (MaterialID :type Integer))
  (bind _output_get (Variables|Default|SetMaterialID MaterialID))
  (Rendering|Material|SetMaterial (Variables|Default|GetPlatform) 0 (Utilities|Array|Get(acopy) (Variables|Default|GetMaterials) _output_get))
  (bind _asgi_game_instance (Utilities|Casting|CastToGI_GameInstance (Game|GetGameInstance)))
  (Default|SubscribePlatformtoArray (Variables|/Game/CustomBlueprints/GI_GameInstance.GI_GameInstance_C|GetPlatformManager _asgi_game_instance) (Utilities|Array|Get(acopy) (Variables|Default|GetMaterials) _output_get) self))

(fn ConstructionScript)