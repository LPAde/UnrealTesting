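; Manager that runs a repeating color-match round, setting the player's material to a random platform group's and moving every other group.
; It registers on GI_GameInstance and sorts subscribing platforms into groups by material.
; A Timeline times each round: on finish it switches the material, waits a delay, moves the non-matching groups and restarts.
; Speed increases periodically by round count, also adjusting the Timeline's play rate.
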(event Custom|SubscribePlatformToArray
  (params (PlatformMaterial :type Material%20Object%20Reference) (PlatformToSubscribe :type BP%20Platform%20Object%20Reference))
  (bind _array_element (Utilities|Array|ForEachLoopwithBreak (Variables|Default|GetPlatforms) :!label _label)
    (:LoopBody
      (if (== (Variables|/Game/CustomBlueprints/BP_PlatformColorHandler.BP_PlatformColorHandler_C|GetManagedMaterial _array_element) PlatformMaterial)
        (Default|AddPlatformtoArray _array_element PlatformToSubscribe)
        (goto _label Break)))))

(event Custom|CheckSpeedIncrease
  (bind _result (Math|Integer|IncrementInt (Variables|Default|GetSpeedIncreaseIndex))
    (:%20%20
      (if (== (Math|Integer|%(Integer) _result (Variables|Default|GetSpeedIncreaseIdentifier)) 0)
        (bind _output_get (Variables|Default|SetCurrentSpeed (+ (Variables|Default|GetCurrentSpeed) (Variables|Default|GetSpeedIncreasesValue))))
        (CallFunction|ChangeTimelinePlayrate _output_get)))))

(event Custom|ChangeTimelinePlayrate
  (params (duration :type Float%20%28double-precision%29))
  (Components|Timeline|SetPlayRate (Variables|Default|GetTimeline) (- duration (Variables|Default|GetMovementDelay))))

(event EventBeginPlay
  (bind _platforms (Variables|Default|GetPlatforms))
  (bind _returnvalue (Utilities|Array|Length _platforms))
  (bind _asgi_game_instance (Utilities|Casting|CastToGI_GameInstance (Game|GetGameInstance)))
  (Variables|/Game/CustomBlueprints/GI_GameInstance.GI_GameInstance_C|SetPlatformManager _asgi_game_instance self)
  (Timeline|Timeline Play
    (:Finished
      (CallFunction|CheckSpeedIncrease)
      (bind _output_get (Variables|Default|SetRandomNumber (Math|Random|RandomInteger _returnvalue)))
      (Default|SetMaterial (Variables|Default|GetPlayer) (Variables|/Game/CustomBlueprints/BP_PlatformColorHandler.BP_PlatformColorHandler_C|GetManagedMaterial (Utilities|Array|Get(acopy) (Variables|Default|GetPlatforms) _output_get)))
      (Utilities|FlowControl|Delay (Variables|Default|GetMovementDelay))
      (for _index (range 0 (- _returnvalue 1))
        (if (not (== _index (Variables|Default|GetRandomNumber)))
          (Default|MovePlatforms (Utilities|Array|Get(acopy) (Variables|Default|GetPlatforms) _index) (Variables|Default|GetCurrentSpeed))))
      (Utilities|FlowControl|Sequence
        (:then_1
          (Timeline|Timeline PlayFromStart))))))

(fn ConstructionScript)